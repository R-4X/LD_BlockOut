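; BP_Key is an interactable key pickup that opens a linked door.
; On Interact, if DoorToOpen is valid, it hides both the door and its own mesh, disables collision on both, and plays a 2D pickup sound.
; Neither actor is destroyed, and the IsLocked and IsInteractionRemoved queries always return false.
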(event `/Game/BPI_Interact.Interact`
  (bind _doortoopen (`self.DoorToOpen`))
  (if (`KismetSystemLibrary.IsValid` _doortoopen)
    (`SceneComponent.SetVisibility` (`Actor.RootComponent` _doortoopen) false true)
    (`self.SetActorEnableCollision` _doortoopen false)
    (`SceneComponent.SetVisibility` (`self.KeyMain`) false true)
    (`self.SetActorEnableCollision` false)
    (`GameplayStatics.PlaySound2D` "/Game/Audio/Key/SFX_KeyPickup.SFX_KeyPickup" 1.0 1.0 0.0 null null)))

(fn `IsInteractionRemoved`
  (returns (IsInteractionRemoved :type Boolean))
  (return false))

(fn `IsLocked`
  (returns (Locked :type Boolean))
  (return false))

(fn `UserConstructionScript`)